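; Base dialogue component for NPC conversations that opens the W_Dialouge widget and notifies its owner on close.
; Child components override the empty Dialogue function, which re-runs from a reset index whenever the conversation progresses.
; AddDialogue replays choices saved in the DialogueProgress map or pushes the first unanswered line to the widget with NPC mood and tree index.
; Helpers clear progress, switch trees and report faction standing toward the player.
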(fn OpenConversation
  (bind _returnvalue (UserInterface|CreateWidget "/Game/UI/W_Dialouge.W_Dialouge_C" 0 self))
  (bind _output_get (Variables|Default|SetDialougeWidget _returnvalue))
  (UserInterface|Viewport|AddtoViewport _output_get 0)
  (CallFunction|ProgressDialogue))

(fn CloseConversation
  (Widget|RemovefromParent (Variables|Default|GetDialougeWidget))
  (Class|BPInteractable|ConvosationClosed(Message) (Components|GetOwner)))

(fn ProgressDialogue
  (Variables|Default|SetDialogueIndex (- (* (Variables|Default|GetQuestionNumber) 2) 1))
  (CallFunction|Dialogue))

(fn Dialogue)

(fn AddDialogue
  (params (Speaker :type Text) (Dialogue :type Text) (OptionText :type Array%20of%20Texts))
  (bind _dialogueprogress (Variables|Default|GetDialogueProgress))
  (bind _dialogueindex (Variables|Default|GetDialogueIndex))
  (bind (_value _returnvalue) (Utilities|Map|Find _dialogueprogress _dialogueindex))
  (Math|Integer|IncrementInt (Variables|Default|GetDialogueIndex)
    (:%20%20
      (if _returnvalue
        (return "NewEnumerator0" _value)
        (else
          (Default|UpdateDialougeText (Variables|Default|GetDialougeWidget) (Variables|Default|GetDialogueIndex) Speaker Dialogue OptionText (Variables|Default|GetNPCShortTermReaction) (Variables|Default|GetDialouge%20Tree%20Index))
          (return "NewEnumerator1" 0))))))

(fn UpdateSelectedOption
  (params (ProgressIndex :type Integer%20%28by%20ref%29) (OptionIndex :type Integer%20%28by%20ref%29))
  (Utilities|Map|Add (Variables|Default|GetDialogueProgress) ProgressIndex OptionIndex)
  (CallFunction|ProgressDialogue))

(fn ClearDialogueProgress
  (Utilities|Map|Clear (Variables|Default|GetDialogueProgress)))

(fn RemoveDialogueProgress
  (params (ProgressStepts :type Integer))
  (for _index (range 0 ProgressStepts)
    (Utilities|Map|Remove (Variables|Default|GetDialogueProgress) (- (Variables|Default|GetDialogueIndex) _index))))

(fn SetDialogueTreeIndex
  (params (DialougeTreeIndex :type FriendType%20Enum :default "NewEnumerator0"))
  (Variables|Default|SetDialouge%20Tree%20Index DialougeTreeIndex)
  (CallFunction|ClearDialogueProgress))

(fn GetFactionInfo
  (bind _faction (Class|BPInteractable|GetFaction(Message) (Components|GetOwner)))
  (bind _factionstate (CallFunction|GetFactionRelationshipRank _faction "/Game/Factions/DataAssets/Factions/Faction_Player.Faction_Player"))
  (return _faction _factionstate))