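; Steve's NPC dialogue, a branching knight-quest conversation whose answers shift his friendship with the player.
; BeginPlay hard-codes a question set per friendship tier, which Dialogue serves one question at a time.
; Each answer's tone, tier, a random mood and faction standing feed the change to NPC_Steve's OverallFriendShip, and also adjust faction relations.
; After a set's last question, that total against a threshold moves the tier up or down.
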(event EventBeginPlay
  (CallFunction|BuildDialogue))

(fn UpdateOverallFrienshipValue
  (params (SetValue :type Integer))
  (bind _returnvalue (Actor|GetActorOfClass "/Game/Blueprints/NPCs/NPC_Steve.NPC_Steve_C"))
  (Variables|/Game/Blueprints/NPCs/NPC_Base.NPC_Base_C|SetOverallFriendShip _returnvalue (+ (Variables|/Game/Blueprints/NPCs/NPC_Base.NPC_Base_C|GetOverallFriendShip _returnvalue) SetValue)))

(fn UpdateShortTermModifier
  (params (CurrentMood :type ENUM_NPCShortTerm%20Enum :default "NewEnumerator0"))
  (switch Utilities|FlowControl|Switch|SwitchonENUM_NPCShortTerm CurrentMood
    (:NewEnumerator0
      (switch Utilities|FlowControl|Switch|SwitchonFriendType (Variables|Default|GetFriendType)
        (:NewEnumerator0
          (bind _output_get (Variables|Default|SetCurrentModifier 4))
          (return _output_get))
        (:NewEnumerator1
          (bind _output_get_2 (Variables|Default|SetCurrentModifier 8))
          (return _output_get_2))
        (:NewEnumerator2
          (bind _output_get_3 (Variables|Default|SetCurrentModifier 10))
          (return _output_get_3))
        (:NewEnumerator3
          (bind _output_get_4 (Variables|Default|SetCurrentModifier 12))
          (return _output_get_4))
        (:NewEnumerator4
          (bind _output_get_5 (Variables|Default|SetCurrentModifier 13))
          (return _output_get_5))
        (:NewEnumerator5
          (bind _output_get_6 (Variables|Default|SetCurrentModifier 15))
          (return _output_get_6))))
    (:NewEnumerator1
      (switch Utilities|FlowControl|Switch|SwitchonFriendType (Variables|Default|GetFriendType)
        (:NewEnumerator0
          (bind _output_get_7 (Variables|Default|SetCurrentModifier 2))
          (return _output_get_7))
        (:NewEnumerator1
          (bind _output_get_8 (Variables|Default|SetCurrentModifier 4))
          (return _output_get_8))
        (:NewEnumerator2
          (bind _output_get_9 (Variables|Default|SetCurrentModifier 6))
          (return _output_get_9))
        (:NewEnumerator3
          (bind _output_get_10 (Variables|Default|SetCurrentModifier 8))
          (return _output_get_10))
        (:NewEnumerator4
          (bind _output_get_11 (Variables|Default|SetCurrentModifier 10))
          (return _output_get_11))
        (:NewEnumerator5
          (bind _output_get_12 (Variables|Default|SetCurrentModifier 12))
          (return _output_get_12))))
    (:NewEnumerator2
      (switch Utilities|FlowControl|Switch|SwitchonFriendType (Variables|Default|GetFriendType)
        (:NewEnumerator0
          (bind _output_get_13 (Variables|Default|SetCurrentModifier -10))
          (return _output_get_13))
        (:NewEnumerator1
          (bind _output_get_14 (Variables|Default|SetCurrentModifier -5))
          (return _output_get_14))
        (:NewEnumerator2
          (bind _output_get_15 (Variables|Default|SetCurrentModifier -1))
          (return _output_get_15))
        (:NewEnumerator3
          (bind _output_get_16 (Variables|Default|SetCurrentModifier 2))
          (return _output_get_16))
        (:NewEnumerator4
          (bind _output_get_17 (Variables|Default|SetCurrentModifier 4))
          (return _output_get_17))
        (:NewEnumerator5
          (bind _output_get_18 (Variables|Default|SetCurrentModifier 6))
          (return _output_get_18))))))

(fn BuildDialogue
  ;[1 1 1] UnFriendly
  (Utilities|Map|Add (Variables|Default|GetDialogueMap) "NewEnumerator0" (Utilities|Struct|MakeQuestions (Utilities|Array|MakeArray (Utilities|Struct|MakeQuestion "\"Do you even have a purpose in this quest, or are you just dead weight?\"" (Utilities|Array|MakeArray (Utilities|Struct|MakeAnswer "\"I get it, I’ve been a liability. But I’m done with that. I’ve got something to prove.\"" "\"You better have a good plan, because right now I’m not convinced.\"") (Utilities|Struct|MakeAnswer "\"I do what I’m told, just like you.\"" "\"That’s your problem, doing what you're told instead of thinking for yourself.\"") (Utilities|Struct|MakeAnswer "\"I don’t need a ‘purpose.’ I’m here because I have to be.\"" "\"Not really helping yourself here.\""))) (Utilities|Struct|MakeQuestion "\"Do you really think you’re capable of winning this fight, or are you just pretending?\"" (Utilities|Array|MakeArray (Utilities|Struct|MakeAnswer "\"I won’t lie, I’ve had my failures. But I’m ready to give everything I’ve got now. I want to fight beside you.\"" "\"You’d better make sure you don’t mess this up. One slip-up and we’re done.\"") (Utilities|Struct|MakeAnswer "\"I’ve got a good chance, but it depends on what we’re up against.\"" "\"Not sure you’ll be much help. We’ll see.\"") (Utilities|Struct|MakeAnswer "\"I’m capable enough. What’s it to you?\"" "\"Not much. Just don’t hold me back.\""))) (Utilities|Struct|MakeQuestion "\"Why are you even still around if you clearly don’t want to be here?\"" (Utilities|Array|MakeArray (Utilities|Struct|MakeAnswer "\"I know I’ve been distant. But I’m staying because I still care about what happens to this team, even if you don’t believe me.\"" "\"You’d better show it, or we’re cutting ties for good.\"") (Utilities|Struct|MakeAnswer "\"I signed up for this, so I’m not backing out now.\"" "\"Well, don’t get in the way then.\"") (Utilities|Struct|MakeAnswer "\"I’m here because I have no choice. You happy now?\"" "\"Not really. Would’ve preferred you stayed home.\""))) (Utilities|Struct|MakeQuestion "\"Do you even try to make a difference, or do you just go through the motions?\"" (Utilities|Array|MakeArray (Utilities|Struct|MakeAnswer "\"I’ve been going through the motions, but I’m done with that. I want to make things right, starting now.\"" "\"You better actually try, or we’ll be in trouble.\"") (Utilities|Struct|MakeAnswer "\"I do what I can. It’s not always about making a big impact.\"" "\"Yeah, but it’s sure easy to forget you’re even here.\"") (Utilities|Struct|MakeAnswer "\"I’m doing what I need to survive. Nothing more.\"" "\"Great, good luck with that.\""))) (Utilities|Struct|MakeQuestion "\"What’s your endgame here? Just survive? Is that really all you’ve got?\"" (Utilities|Array|MakeArray (Utilities|Struct|MakeAnswer "\"Survive? No, I want to leave my mark. I want to prove I’m more than just another knight.\"" "\"Prove it. You’ve got one chance.\"") (Utilities|Struct|MakeAnswer "\"My endgame is finishing this quest. Then we’ll see.\"" "\"That’s not exactly reassuring, but okay.\"") (Utilities|Struct|MakeAnswer "\"Surviving. That’s all. Don’t expect anything more.\"" "\"Can’t wait for you to make that your excuse when it all falls apart.\""))))))
  ;[1 1 1] UnFriendly
  (Utilities|Map|Add (Variables|Default|GetDialogueMap) "NewEnumerator1" (Utilities|Struct|MakeQuestions (Utilities|Array|MakeArray (Utilities|Struct|MakeQuestion "\"What do you think you’re even good at, aside from getting in the way?\"" (Utilities|Array|MakeArray (Utilities|Struct|MakeAnswer "\"I know I’ve messed up before, but I can still be useful. Let me prove it to you.\"" "\"Yeah, well, you’d better. I’m not sticking around if you keep dragging your feet.\"") (Utilities|Struct|MakeAnswer "\"I get the job done. Enough said.\"" "\"Hope you can keep it that way.\"") (Utilities|Struct|MakeAnswer ": \"I’m not here to impress you.\"" "\"Not like I asked you to. Just try not to mess things up.\""))) (Utilities|Struct|MakeQuestion "\"What makes you think you’re qualified to lead anyone?\"" (Utilities|Array|MakeArray (Utilities|Struct|MakeAnswer "\"I know I haven’t always stepped up, but I’m willing to try if you’ll give me a chance.\"" "\"If you actually step up this time, maybe you’ll prove me wrong.\"") (Utilities|Struct|MakeAnswer "\"I’ve been in charge before. It’s not that hard.\"" "\"We’ll see how long that lasts.\"") (Utilities|Struct|MakeAnswer "\"I don’t care about leading. I just do my part.\"" "\"Well, I hope your part isn’t getting us all killed.\""))) (Utilities|Struct|MakeQuestion "\"Ever get tired of just being... here? No ambition or anything?\"" (Utilities|Array|MakeArray (Utilities|Struct|MakeAnswer "\"I know I’ve been stagnant. But I want to change that. I’m in this for the long haul now.\"" "\"You better mean it this time.\"") (Utilities|Struct|MakeAnswer "\"I get by. Ambition’s overrated anyway.\"" "\"Not if you want to actually get somewhere.\"") (Utilities|Struct|MakeAnswer "\"No. I’m just doing what I need to survive.\"" "\"Great. Keep that low effort to yourself.\""))) (Utilities|Struct|MakeQuestion "\"Ever get tired of just being... here? No ambition or anything?\"" (Utilities|Array|MakeArray (Utilities|Struct|MakeAnswer "\"I won’t give up. Not now, not ever. I’ll fight with everything I’ve got.\"" "\"If you show that kind of determination, maybe you’ll redeem yourself.\"") (Utilities|Struct|MakeAnswer "\"We’ll see. Nothing’s ever certain.\"" "\"That’s not exactly reassuring, but okay.\"") (Utilities|Struct|MakeAnswer "\"I’ll survive. That’s all that matters.\"" "\"Great, good luck with that.\""))) (Utilities|Struct|MakeQuestion "\"Do you even care about what happens to the others, or is it just about you?\"" (Utilities|Array|MakeArray (Utilities|Struct|MakeAnswer "\"I know I’ve been selfish in the past, but I care. I’ll prove it to you. We’re a team.\"" "\"I’ll believe it when I see it.\"") (Utilities|Struct|MakeAnswer "\"I care about the outcome. That’s all.\"" "\"Right, as long as it doesn’t inconvenience you.\"") (Utilities|Struct|MakeAnswer "\"I don’t care about anyone else.\"" "\"I figured. It shows.\""))))))
  ;[1 1 1] Casual
  (Utilities|Map|Add (Variables|Default|GetDialogueMap) "NewEnumerator2" (Utilities|Struct|MakeQuestions (Utilities|Array|MakeArray (Utilities|Struct|MakeQuestion "\"So, how long have you been on the path of a knight?\"" (Utilities|Array|MakeArray (Utilities|Struct|MakeAnswer "\"Since forever! Can you believe they still haven't promoted me yet?\"" "\"Sounds like we need to cause some commotion to get you noticed!\"") (Utilities|Struct|MakeAnswer "\"A few years. It’s been a decent life.\"" "\"Fair enough. Guess we all have our reasons.\"") (Utilities|Struct|MakeAnswer "\"Long enough to know when to keep to myself.\"" "\"Understood. No need to dig deeper.\""))) (Utilities|Struct|MakeQuestion "\"What brings you to this quest, anyway?" (Utilities|Array|MakeArray (Utilities|Struct|MakeAnswer "\"You know, the usual—glory, treasure, and hopefully a good story!\"" "\"Then let’s make sure it’s a tale worth telling!\"") (Utilities|Struct|MakeAnswer "\"The coin is decent, and the work’s honorable.\"" "\"Good enough for me. We’ll see it through together.\"") (Utilities|Struct|MakeAnswer "\"That's my business, not yours.\"" "\"Fine. Just curious.\""))) (Utilities|Struct|MakeQuestion "\"Do you have any special skills in battle?\"" (Utilities|Array|MakeArray (Utilities|Struct|MakeAnswer "\"Well, I think I could teach you a thing or two!\"" "\"Now you’re speaking my language! Show me what you’ve got!\"") (Utilities|Struct|MakeAnswer "\"A few. I’m decent with a longsword.\"" "\"Good to know. We’ll watch each other’s backs.\"") (Utilities|Struct|MakeAnswer "\"Why? Planning to copy my moves?\"" "\"Relax, just trying to size up my ally.\""))) (Utilities|Struct|MakeQuestion "\"Ever fought a dragon before?\"" (Utilities|Array|MakeArray (Utilities|Struct|MakeAnswer "\"Not yet, but I'm ready when you are!\"" "\"Well, here’s hoping today’s the day!\"") (Utilities|Struct|MakeAnswer "\"No, but I’ve prepared for it.\"" "\"That’s all we can do, I suppose.\"") (Utilities|Struct|MakeAnswer "\"Why would I tell you?\"" "\"Keep your secrets, then.\""))) (Utilities|Struct|MakeQuestion "\"What's your weapon of choice?\"" (Utilities|Array|MakeArray (Utilities|Struct|MakeAnswer "\"My sword—and, of course, a trusty sidekick like you!\"" "\"I knew you’d say that! The perfect duo!\"") (Utilities|Struct|MakeAnswer "\"A sword. Gets the job done.\"" "\"Classic choice. I can respect that.\"") (Utilities|Struct|MakeAnswer "\"What difference does it make to you?\"" "\"Noted. No need to get prickly.\""))))))
  ;[1 1 1] Friendly
  (Utilities|Map|Add (Variables|Default|GetDialogueMap) "NewEnumerator3" (Utilities|Struct|MakeQuestions (Utilities|Array|MakeArray (Utilities|Struct|MakeQuestion "\"Do you believe in all those knightly codes and vows?\"" (Utilities|Array|MakeArray (Utilities|Struct|MakeAnswer "\"Only when it’s convenient—don’t tell the guild!\"" "\"Ha! Our little secret, then.\"") (Utilities|Struct|MakeAnswer "\"They have their place, I suppose.\"" "\"Good enough answer for me.\"") (Utilities|Struct|MakeAnswer "\"What I believe isn’t your concern.\"" "\"Point taken. Let’s keep it moving.\""))) (Utilities|Struct|MakeQuestion "\"Think we’ll actually get a reward for this quest?\"" (Utilities|Array|MakeArray (Utilities|Struct|MakeAnswer "\"If not, you and I are taking what we’re owed, right?\"" "\"Absolutely! No one cheats this team!\"") (Utilities|Struct|MakeAnswer "\"I expect we will, if all goes well.\"" "\"Let’s get it done, then.\"") (Utilities|Struct|MakeAnswer "\"I don't care about rewards.\"" "\"Suit yourself, then.\""))) (Utilities|Struct|MakeQuestion "\"What’s your favorite battle tactic?\"" (Utilities|Array|MakeArray (Utilities|Struct|MakeAnswer "\"Sticking close to you—no one takes us down together!\"" "\"The unbeatable combo! Let’s keep it that way!\"") (Utilities|Struct|MakeAnswer "\"Stay on the defense, then look for an opening.\"" "\"Sounds smart. I’ll keep my guard up, too.\"") (Utilities|Struct|MakeAnswer "\"I’m not giving away my strategy.\"" "\"No problem. Keep your secrets.\""))) (Utilities|Struct|MakeQuestion "\"Are you superstitious? You know, about enchanted armor or cursed amulets?\"" (Utilities|Array|MakeArray (Utilities|Struct|MakeAnswer "\"Absolutely! Why risk it? Besides, it makes for a good story.\"" "\"True! We’ll keep our luck on our side!\"") (Utilities|Struct|MakeAnswer "\"Not really, but it pays to be cautious.\"" "\"That’s fair. Better safe than sorry.\"") (Utilities|Struct|MakeAnswer "\"No. Don’t believe in that nonsense.\"" "\"All right, all right. Just wondering.\""))) (Utilities|Struct|MakeQuestion "\"Ever thought about retiring from all this?\"" (Utilities|Array|MakeArray (Utilities|Struct|MakeAnswer "\"Only if you retire with me. Can’t let you have all the glory!\"" "\"Deal! We’ll toast to it one day!\"") (Utilities|Struct|MakeAnswer "\"Once or twice, maybe. It’s crossed my mind.\"" "\"I get that. But there’s still work to be done.\"") (Utilities|Struct|MakeAnswer "\"No.\"\"" "\"Fair enough.\""))))))
  ;[1 1 1] Close Friends
  (Utilities|Map|Add (Variables|Default|GetDialogueMap) "NewEnumerator4" (Utilities|Struct|MakeQuestions (Utilities|Array|MakeArray (Utilities|Struct|MakeQuestion "\"What’s the toughest foe you've faced so far?\"" (Utilities|Array|MakeArray (Utilities|Struct|MakeAnswer "\"That wild boar last winter—still laugh about that, don’t we?\"" "\"Can’t believe we made it out of that mess!\"") (Utilities|Struct|MakeAnswer "\"Probably a brigand leader last spring. Skilled, but reckless.\"" "\"Good one. I’ll keep an eye out for those types.\"") (Utilities|Struct|MakeAnswer "\"I don’t keep track.\"" "\"All right, moving on.\""))) (Utilities|Struct|MakeQuestion "\"Do you trust everyone in the party?\"" (Utilities|Array|MakeArray (Utilities|Struct|MakeAnswer "\"Only you, honestly. The others seem a bit shady, don’t you think?\"" "\"Couldn’t agree more. Let’s watch each other’s backs.\"") (Utilities|Struct|MakeAnswer "\"Mostly, but I keep an eye open just in case.\"" "\"That’s smart. I’ll do the same.\"") (Utilities|Struct|MakeAnswer "\"I trust no one.\"" "\"Noted. I’ll keep to myself.\""))) (Utilities|Struct|MakeQuestion "\"What do you do to keep your spirits up when things get tough?\"" (Utilities|Array|MakeArray (Utilities|Struct|MakeAnswer "\"Having you around helps—can’t have the serious knight without the joker!\"" "\"Right back at you. We keep each other going.\"") (Utilities|Struct|MakeAnswer "\"I focus on the task and try not to dwell.\"" "\"Makes sense. Stay sharp, right?\"") (Utilities|Struct|MakeAnswer "\"Don’t need anything to keep my spirits up.\"" "\"All right, stoic as ever.\""))) (Utilities|Struct|MakeQuestion "\"Ever regret choosing the path of a knight?\"" (Utilities|Array|MakeArray (Utilities|Struct|MakeAnswer "\"Nah! Not with you along for the ride.\"" "\"Same here! Here’s to more adventures together.\"") (Utilities|Struct|MakeAnswer "\"Sometimes, but I wouldn’t change it.\"" "\"Wise answer. No going back now.\"") (Utilities|Struct|MakeAnswer "\"Why does it matter to you?\"" "\"Just curious.\""))) (Utilities|Struct|MakeQuestion "\"What do you think lies beyond this forest?\"" (Utilities|Array|MakeArray (Utilities|Struct|MakeAnswer "\"Treasure, fame, and an epic battle waiting for us both!\"" "\"Can’t wait! I’m right by your side!\"") (Utilities|Struct|MakeAnswer "\"Not sure. Perhaps a hidden village or an enemy camp.\"" "\"Either way, we’ll be ready.\"") (Utilities|Struct|MakeAnswer "\"Doesn’t matter until we get there.\"" "\"Fair enough.\""))))))
  ;[1 1 1] Best Friends
  (Utilities|Map|Add (Variables|Default|GetDialogueMap) "NewEnumerator5" (Utilities|Struct|MakeQuestions (Utilities|Array|MakeArray (Utilities|Struct|MakeQuestion "\"Do you think we’ll both survive this quest?\"" (Utilities|Array|MakeArray (Utilities|Struct|MakeAnswer "\"Of course! As long as I have you by my side, we’re unstoppable!\"" "\"I trust you. Let’s make it back together!\"") (Utilities|Struct|MakeAnswer "\"I hope so, but nothing’s certain.\"" " \"We’ll see it through.\"") (Utilities|Struct|MakeAnswer "\"I’ll survive. That’s all I need to worry about.\"" "\"Guess it’s everyone for themselves, then.\""))) (Utilities|Struct|MakeQuestion "\"What will you do if we find the lost kingdom we’re searching for?\"" (Utilities|Array|MakeArray (Utilities|Struct|MakeAnswer "\"Build you a throne right next to mine!\"" "\"Couldn’t agree more. Let’s watch each other’s backs.\"") (Utilities|Struct|MakeAnswer "\"Accept whatever fate has planned for me.\"" "\"That’s smart. I’ll do the same.\"") (Utilities|Struct|MakeAnswer "\"I’ll claim my reward and leave.\"" "\"Noted. I’ll keep to myself.\""))) (Utilities|Struct|MakeQuestion "\"If we get separated in battle, what should I do?\"" (Utilities|Array|MakeArray (Utilities|Struct|MakeAnswer "\"Stick to the plan and meet me back here—nothing’s keeping us apart.\"" "\"Deal. I’ll always find my way back to you.\"") (Utilities|Struct|MakeAnswer "\"Continue the mission, I suppose.\"" "\"All right, mission first.\"") (Utilities|Struct|MakeAnswer "\"That’s up to you. I don’t need rescuing.\"" "\"Understood. You’re on your own, then.\""))) (Utilities|Struct|MakeQuestion "\"Do you think we’ll stay close after this quest ends?\"" (Utilities|Array|MakeArray (Utilities|Struct|MakeAnswer "We’ll be legends together! Partners for life, right?\"" "\"Absolutely! Together till the end!\"") (Utilities|Struct|MakeAnswer "\"Perhaps. It depends on where the road leads.\"" "\"I guess time will tell.\"") (Utilities|Struct|MakeAnswer "\"Doubt it.\"" "\"Suit yourself.\""))) (Utilities|Struct|MakeQuestion "\"If one of us doesn’t make it, what would you want me to do?\"" (Utilities|Array|MakeArray (Utilities|Struct|MakeAnswer "\"Tell everyone our story—and don’t let anyone forget me!\"" "\"You’ll be remembered, trust me on that.\"") (Utilities|Struct|MakeAnswer "\"Fulfill the quest and move on.\"" "\"I’ll honor that.\"") (Utilities|Struct|MakeAnswer "\"Forget me and keep moving.\"" "\"Will do.\"")))))))

(fn Dialogue
  (bind _currentanswer (Variables|Default|GetCurrentAnswer))
  ;[1 1 1] Comment
  (|CallParentFunction)
  (Utilities|Array|Clear (Variables|Default|GetCurrentAnswer))
  (for _array_element (.Answers (Utilities|Struct|BreakQuestion (Utilities|Array|Get(acopy) (Utilities|Struct|BreakQuestions (.Value (Utilities|Map|Find (Variables|Default|GetDialogueMap) (Variables|Default|GetFriendType)))) (Variables|Default|GetQuestionNumber))))
    (Utilities|Array|Add _currentanswer (.Answer (Utilities|Struct|BreakAnswer _array_element))))
  (bind (_state _optionindex) (CallFunction|AddDialogue "Steve" (.Question (Utilities|Struct|BreakQuestion (Utilities|Array|Get(acopy) (Utilities|Struct|BreakQuestions (.Value (Utilities|Map|Find (Variables|Default|GetDialogueMap) (Variables|Default|GetFriendType)))) (Variables|Default|GetQuestionNumber)))) _currentanswer))
  (switch Utilities|FlowControl|Switch|SwitchonEnum_progress_DialogueState _state
    (:NewEnumerator0
      (bind _state_2 (CallFunction|AddDialogue "Steve" (.Reply (Utilities|Struct|BreakAnswer (Utilities|Array|Get(acopy) (.Answers (Utilities|Struct|BreakQuestion (Utilities|Array|Get(acopy) (Utilities|Struct|BreakQuestions (.Value (Utilities|Map|Find (Variables|Default|GetDialogueMap) (Variables|Default|GetFriendType)))) (Variables|Default|GetQuestionNumber)))) _optionindex))) (Utilities|Array|MakeArray "Continue")))
      (switch Utilities|FlowControl|Switch|SwitchonEnum_progress_DialogueState _state_2
        (:NewEnumerator0
          _)
        (:NewEnumerator1
          (Math|Integer|IncrementInt (Variables|Default|GetQuestionNumber)
            (:%20%20
              (switch int _optionindex
                (:0
                  (Variables|Default|SetNPCShortTermReaction "NewEnumerator0")
                  (bind _factionmodifier (CallFunction|GetfactionModifier))
                  (bind _shorttermmodifier (CallFunction|UpdateShortTermModifier (Variables|Default|GetNPCShortTermReaction)))
                  (bind _randommoodmodifiervalue (CallFunction|RandomMoodModifier))
                  (bind _outpulvalue (CallFunction|CalculateFriendShipChangeValue _randommoodmodifiervalue _shorttermmodifier (Variables|Default|GetPositiveSpeachInpactModifier) _factionmodifier))
                  (CallFunction|UpdateOverallFrienshipValue _outpulvalue)
                  (CallFunction|UpdateFaction 5))
                (:1
                  (Variables|Default|SetNPCShortTermReaction "NewEnumerator1")
                  (bind _factionmodifier_2 (CallFunction|GetfactionModifier))
                  (bind _shorttermmodifier_2 (CallFunction|UpdateShortTermModifier (Variables|Default|GetNPCShortTermReaction)))
                  (bind _randommoodmodifiervalue_2 (CallFunction|RandomMoodModifier))
                  (bind _outpulvalue_2 (CallFunction|CalculateFriendShipChangeValue _randommoodmodifiervalue_2 _shorttermmodifier_2 (Variables|Default|GetNeturalSpeachInpactModifier) _factionmodifier_2))
                  (CallFunction|UpdateOverallFrienshipValue _outpulvalue_2)
                  (CallFunction|UpdateFaction 2))
                (:2
                  (Variables|Default|SetNPCShortTermReaction "NewEnumerator2")
                  (bind _factionmodifier_3 (CallFunction|GetfactionModifier))
                  (bind _shorttermmodifier_3 (CallFunction|UpdateShortTermModifier (Variables|Default|GetNPCShortTermReaction)))
                  (bind _randommoodmodifiervalue_3 (CallFunction|RandomMoodModifier))
                  (bind _outpulvalue_3 (CallFunction|CalculateFriendShipChangeValue _randommoodmodifiervalue_3 _shorttermmodifier_3 (Variables|Default|GetNegativeSpeachInpactModifier) _factionmodifier_3))
                  (CallFunction|UpdateOverallFrienshipValue _outpulvalue_3)
                  (CallFunction|UpdateFaction -5)))))))
      (if (>= (Variables|Default|GetQuestionNumber) (- (Utilities|Array|Length (Utilities|Struct|BreakQuestions (.Value (Utilities|Map|Find (Variables|Default|GetDialogueMap) (Variables|Default|GetFriendType))))) 1))
        (Variables|Default|SetQuestionNumber 0)
        (bind _returnvalue (Actor|GetActorOfClass "/Game/Blueprints/NPCs/NPC_Steve.NPC_Steve_C"))
        (if (> (Variables|/Game/Blueprints/NPCs/NPC_Base.NPC_Base_C|GetOverallFriendShip _returnvalue) (Variables|Default|GetImproveFrienshipThreshold))
          (CallFunction|ClearDialogueProgress)
          (CallFunction|CloseConversation)
          (if (Utilities|Enum|Equal(Enum) (Variables|Default|GetDialouge%20Tree%20Index) "NewEnumerator5")
            _
            (else
              (bind _result (Math|Integer|IncrementInt (Math|Conversions|ToInteger(Byte) (Variables|Default|GetFriendType)))
                (:%20%20
                  (bind _output_get (Variables|Default|SetFriendType (Utilities|Enum|ByteToEnumFriendType (Math|Conversions|ToByte(Integer) _result))))))))
          (CallFunction|SetDialogueTreeIndex _output_get)
          (else
            (CallFunction|ClearDialogueProgress)
            (CallFunction|CloseConversation)
            (if (Utilities|Enum|Equal(Enum) (Variables|Default|GetDialouge%20Tree%20Index) "NewEnumerator0")
              _
              (else
                (bind _result_2 (Math|Integer|DecrementInt (Math|Conversions|ToInteger(Byte) (Variables|Default|GetFriendType)))
                  (:%20%20
                    (bind _output_get_2 (Variables|Default|SetFriendType (Utilities|Enum|ByteToEnumFriendType (Math|Conversions|ToByte(Integer) _result_2))))))))
            (CallFunction|SetDialogueTreeIndex _output_get_2)))))))

(fn RandomMoodModifier
  (bind _moodlist (Variables|Default|GetMoodList))
  (bind _output_get (LocalVariables|SetCurrentMood (Utilities|Array|Get(acopy) _moodlist (Math|Random|RandomIntegerinRange 0 (Utilities|Array|LastIndex _moodlist)))))
  (switch Utilities|FlowControl|Switch|SwitchonMoodList _output_get
    (:NewEnumerator0
      (return 10))
    (:NewEnumerator1
      (return 8))
    (:NewEnumerator2
      (return 6))
    (:NewEnumerator3
      (return 4))
    (:NewEnumerator4
      (return 2))
    (:NewEnumerator5
      (return -2))
    (:NewEnumerator6
      (return -4))
    (:NewEnumerator7
      (return -6))
    (:NewEnumerator8
      (return -8))
    (:NewEnumerator9
      (return -10))))

(fn CalculateFriendShipChangeValue
  (params (NPC_CurrentMoodValue :type Integer) (ResponceImpact :type Integer) (TypeOfResponce :type Integer) (FactionModifier :type Integer))
  ;[1 1 1] convert to floats for math
  (LocalVariables|SetMood (Math|Conversions|ToFloat(Integer) NPC_CurrentMoodValue))
  (LocalVariables|SetImpact (Math|Conversions|ToFloat(Integer) ResponceImpact))
  (LocalVariables|SetResponce (Math|Conversions|ToFloat(Integer) TypeOfResponce))
  (LocalVariables|SetFactionMod (Math|Conversions|ToFloat(Integer) FactionModifier))
  ;[1 1 1] Branch Nodes to determine ResponseType conditions (positive, negative, neutral).
  (if (> (LocalVariables|GetResponce) 0.0)
    ;[1 1 1] Math Nodes for division and addition to calculate AdjustmentFactor
    (LocalVariables|SetAdjustmentFactor (+ (/ (* (LocalVariables|GetResponce) (LocalVariables|GetImpact)) 1e+01) 1.0))
    (elif (< (LocalVariables|GetResponce) 0.0)
      (LocalVariables|SetAdjustmentFactor (+ (/ (* (LocalVariables|GetResponce) (LocalVariables|GetImpact)) 2e+01) 1.0))
      (else
        (LocalVariables|SetAdjustmentFactor 1.0))))
  ;[1 1 1] Multiply and Add Nodes to combine inputs and calculate the final output. (if found two negatives times results by a negitive to give true repersentation)
  (if (and (< (LocalVariables|GetResponce) 0.0) (< (LocalVariables|GetAdjustmentFactor) 0.0))
    (return (Math|Float|Truncate (+ (* (* (LocalVariables|GetResponce) (Math|Float|Clamp(Float) (LocalVariables|GetAdjustmentFactor) (Math|Random|RandomFloatinRange 0.1 1.0) 1e+02)) 1.0) (/ (LocalVariables|GetFactionMod) (Variables|Default|GetFactionLoyalty)))))
    (else
      (return (Math|Float|Truncate (+ (/ (+ (* (LocalVariables|GetResponce) (Math|Float|Clamp(Float) (LocalVariables|GetAdjustmentFactor) 0.01 1e+02)) (LocalVariables|GetMood)) 25.0) (/ (LocalVariables|GetFactionMod) (Variables|Default|GetFactionLoyalty))))))))

(fn UpdateFaction
  (params (Relationship :type Integer))
  (bind _faction (Class|BPInteractable|GetFaction(Message) (Game|GetPlayerCharacter 0)))
  (bind _faction_2 (Class|BPInteractable|GetFaction(Message) (Components|GetOwner)))
  (CallFunction|UpdateFactionRelationship _faction_2 _faction Relationship))

(fn GetfactionModifier
  (bind _faction (Class|BPInteractable|GetFaction(Message) (Components|GetOwner)))
  (bind _faction_2 (Class|BPInteractable|GetFaction(Message) (Game|GetPlayerCharacter 0)))
  (bind _factionstate (CallFunction|GetFactionRelationshipRank _faction _faction_2))
  (switch Utilities|FlowControl|Switch|Switchone_FactionStates _factionstate
    (:NewEnumerator0
      (bind _output_get (Variables|Default|SetCalculateFactionModifier 4))
      (return _output_get))
    (:NewEnumerator1
      (bind _output_get_2 (Variables|Default|SetCalculateFactionModifier 2))
      (return _output_get_2))
    (:NewEnumerator2
      (bind _output_get_3 (Variables|Default|SetCalculateFactionModifier 0))
      (return _output_get_3))
    (:NewEnumerator3
      (bind _output_get_4 (Variables|Default|SetCalculateFactionModifier -2))
      (return _output_get_4))
    (:NewEnumerator4
      (bind _output_get_5 (Variables|Default|SetCalculateFactionModifier -4))
      (return _output_get_5))))