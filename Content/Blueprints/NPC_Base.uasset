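; Base NPC Blueprint that carries a character name and a faction, with hooks for interaction and conversation.
; The construction script writes the name to a text component, which SetInteractableState shows or hides as interaction availability changes.
; When a conversation closes, it forwards that notification to the stored interaction instigator.
; GetFaction exposes the NPC's faction.
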(event EventSetInteractableState
  (params (bCanShowInteract :type Boolean))
  (if bCanShowInteract
    (Rendering|SetVisibility (Variables|Default|GetText_CharacterName) true false)
    (else
      (Rendering|SetVisibility (Variables|Default|GetText_CharacterName) false false))))

(event EventConvosationClosed
  (Class|BPInteractable|ConvosationClosed(Message) (Variables|Default|GetInteractInstagator)))

(fn ConstructionScript
  (Rendering|Components|TextRender|SetText (Variables|Default|GetText_CharacterName) (Variables|Default|GetCharacterName)))

(fn GetFaction
  (return (Variables|Default|GetFaction)))