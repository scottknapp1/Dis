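; Dialogue Blueprint for NPC Eve, holding draft branching-conversation logic that is currently unreachable, with empty or zero-returning function stubs.
; The unwired graph pulls questions, answers and replies from DialogueMap by FriendType, mapping the chosen option to positive, neutral or negative short-term reputation.
; After the last question, it compares GS_DialougeSystem's short-term score to a threshold, steps FriendType up or down, and resets the dialogue tree.
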(fn UpdateLongTermRep
  (params (ValueSet :type Integer)))

(fn UpdateShortTermRep
  (params (SetValue :type Integer)))

(fn UpdateShortTermModifier
  (params (CurrentMood :type ENUM_NPCShortTerm%20Enum :default "NewEnumerator0"))
  (return 0))

(fn Dialouge)

(fn BuildDialogue)